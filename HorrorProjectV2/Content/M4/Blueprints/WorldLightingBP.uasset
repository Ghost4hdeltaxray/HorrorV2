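; WorldLightingBP is an all-in-one world lighting actor bundling sun, skylight, atmosphere, height fog, volumetric clouds and post process.
; Construction script and BeginPlay both toggle components from booleans and optionally apply simple sun, fog and cloud overrides.
; They also set Lumen and Virtual Shadow Maps through console variables, copying those flags to an EditorHelperBP actor.
; A DisableAllM4Lighting event switches every component off.
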(event Custom|Disable%20All%20M4%20Lighting
  (Rendering|SetVisibility (Variables|Default|GetDirectionalLight) false false)
  (Rendering|SetVisibility (Variables|Default|GetSkyLight) false false)
  (Rendering|SetVisibility (Variables|Default|GetSkyAtmosphere) false false)
  (Rendering|SetVisibility (Variables|Default|GetExponentialHeightFog) false false)
  (Rendering|SetVisibility (Variables|Default|GetVolumetricCloud) false false)
  (Variables|/Script/Engine.PostProcessComponent|SetbEnabled (Variables|Default|GetPostProcess) false)
  (Variables|LightingComponentToggles|SetDirectional%20Light false)
  (Variables|LightingComponentToggles|SetSky%20Light false)
  (Variables|LightingComponentToggles|SetSky%20Atmosphere false)
  (Variables|LightingComponentToggles|SetExponential%20Height%20Fog false)
  (Variables|LightingComponentToggles|SetVolumetric%20Clouds false)
  (Variables|LightingComponentToggles|SetPost%20Process false))

(event EventBeginPlay
  (CallFunction|SetVirtualShadowMaps)
  (CallFunction|SetLumen)
  (CallFunction|ToggleOn/OffComponents)
  (CallFunction|SetSimpleEnvironmentSettings))

(event Collision|EventActorBeginOverlap
  (params (OtherActor :type Actor%20Object%20Reference)))

(event EventTick
  (params (DeltaSeconds :type Float%20%28single-precision%29)))

(fn ConstructionScript
  (CallFunction|SetVirtualShadowMaps)
  (CallFunction|SetLumen)
  (CallFunction|ToggleOn/OffComponents)
  (CallFunction|SetSimpleEnvironmentSettings))

(fn ToggleOn/OffComponents
  (Rendering|SetVisibility (Variables|Default|GetDirectionalLight) (Variables|LightingComponentToggles|GetDirectional%20Light) false)
  (Rendering|SetVisibility (Variables|Default|GetSkyLight) (Variables|LightingComponentToggles|GetSky%20Light) false)
  (Rendering|SetVisibility (Variables|Default|GetSkyAtmosphere) (Variables|LightingComponentToggles|GetSky%20Atmosphere) false)
  (Rendering|SetVisibility (Variables|Default|GetExponentialHeightFog) (Variables|LightingComponentToggles|GetExponential%20Height%20Fog) false)
  (Rendering|SetVisibility (Variables|Default|GetVolumetricCloud) (Variables|LightingComponentToggles|GetVolumetric%20Clouds) false)
  (Variables|/Script/Engine.PostProcessComponent|SetbEnabled (Variables|Default|GetPostProcess) (Variables|LightingComponentToggles|GetPost%20Process)))

(fn SetLumen
  (if (Variables|Lumen&VirtualShadowMaps(Override)|GetEnable%20Lumen)
    (Development|ExecuteConsoleCommand "r.Lumen.DiffuseIndirect.Allow 1" 0)
    (else
      (Development|ExecuteConsoleCommand "r.Lumen.DiffuseIndirect.Allow 0" 0)))
  (bind _returnvalue (Actor|GetActorOfClass "/Game/M4/Blueprints/EditorHelperBP.EditorHelperBP_C"))
  (Utilities|IsValid _returnvalue
    (:Is%20Valid
      (Variables|/Game/M4/Blueprints/EditorHelperBP.EditorHelperBP_C|SetEnable%20Lumen _returnvalue (Variables|Lumen&VirtualShadowMaps(Override)|GetEnable%20Lumen)))))

(fn SetVirtualShadowMaps
  (bind _returnvalue (Development|GetConsoleVariableIntValue "r.Shadow.Virtual.Enable"))
  (Variables|Default|SetEnable%20Virtual%20Shadow%20Maps%20%28Previous%29 (Math|Conversions|ToBoolean(Integer) _returnvalue))
  (if (not (== (Variables|Lumen&VirtualShadowMaps(Override)|GetEnable%20Virtual%20Shadow%20Maps) (Variables|Default|GetEnable%20Virtual%20Shadow%20Maps%20%28Previous%29)))
    (if (Variables|Lumen&VirtualShadowMaps(Override)|GetEnable%20Virtual%20Shadow%20Maps)
      (Development|ExecuteConsoleCommand "r.Shadow.Virtual.Enable 1" 0)
      (else
        (Development|ExecuteConsoleCommand "r.Shadow.Virtual.Enable 0" 0)))
    (bind _returnvalue_2 (Actor|GetActorOfClass "/Game/M4/Blueprints/EditorHelperBP.EditorHelperBP_C"))
    (Utilities|IsValid _returnvalue_2
      (:Is%20Valid
        (Variables|/Game/M4/Blueprints/EditorHelperBP.EditorHelperBP_C|SetEnable%20Virtual%20Shadow%20Maps _returnvalue_2 (Variables|Lumen&VirtualShadowMaps(Override)|GetEnable%20Virtual%20Shadow%20Maps))))))

(fn SetSimpleEnvironmentSettings
  (bind _directionallight (Variables|Default|GetDirectionalLight))
  (bind _exponentialheightfog (Variables|Default|GetExponentialHeightFog))
  (bind _volumetriccloud (Variables|Default|GetVolumetricCloud))
  (if (Variables|SimpleEnvironmentOverrides|GetEnable%20Override%20Settings%20Below)
    (Transformation|SetWorldRotation _directionallight (Math|Rotator|MakeRotator 1.8e+02 (Variables|SimpleEnvironmentOverrides|GetSun%20Angle) (Variables|SimpleEnvironmentOverrides|GetSun%20Rotation)) false false)
    (Rendering|Components|Light|SetIntensity _directionallight (Variables|SimpleEnvironmentOverrides|GetSun%20Intensity))
    (Rendering|Components|Light|SetLightColor _directionallight (Variables|SimpleEnvironmentOverrides|GetSun%20Light%20Color) true)
    (Rendering|Components|Light|SetIntensity (Variables|Default|GetSkyLight) (Variables|SimpleEnvironmentOverrides|GetSkylight%20Intensity))
    (Class|ExponentialHeightFogComponent|SetFogDensity _exponentialheightfog (Variables|SimpleEnvironmentOverrides|GetFog%20Density))
    (Transformation|SetWorldLocation _exponentialheightfog (Math|Vector|MakeVector 0.0 0.0 (Variables|SimpleEnvironmentOverrides|GetFog%20Height)) false false)
    (Class|VolumetricCloudComponent|SetViewSampleCountScale _volumetriccloud (Variables|SimpleEnvironmentOverrides|GetCloud%20Visual%20Quality%20%28Affects%20FPS%29))
    (Class|VolumetricCloudComponent|SetShadowViewSampleCountScale _volumetriccloud (Variables|SimpleEnvironmentOverrides|GetCloud%20Shadow%20Quality%20%28Affects%20FPS%29))))