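; Helper actor that draws terrain trails and foliage trampling into render targets around the player, using settings from TrailsAndTrampleBP.
; Tick finds moved colliders, snaps the capture area to the player's texel grid, updates material parameter collection offsets, then draws temporary, persistent, blurred and terrain normal passes.
; Timed overlap checks gate each system by volume, clearing targets after exit.
; Foliage timers publish player velocity and nudge collider records to force redraws for fading.
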(event Custom|Set%20Direction%20of%20Travel
  (bind _returnvalue (Game|GetPlayerCharacter 0))
  (bind _charactermovement (Variables|/Script/Engine.Character|GetCharacterMovement _returnvalue))
  (bind _returnvalue_2 (Pawn|Components|CharacterMovement|GetLastUpdateVelocity _charactermovement))
  (bind (_x _y) (Math|Vector|BreakVector _returnvalue_2))
  ;[0.0205 0.4638 1] Direction of Travel Detection
  (Utilities|IsValid (Game|GetPlayerCharacter 0)
    (:Is%20Valid
      (if (Math|Vector|NotEqual(Vector) _returnvalue_2 "0, 0, 0" 0.0001)
        (Rendering|Material|SetVectorParameterValue "/Game/M4/Blueprints/SystemResources/Trails/MPCs/TrailCapture.TrailCapture" "PlayerVelocity" (Math|Conversions|ToLinearColor(Vector) (Math|Vector|ClampVectorSize (Math|Vector|MakeVector _x _y 0.0) -2.0 2.0)) :!class /Script/Engine.KismetMaterialLibrary)))))

(event Custom|Volume%20Overlap%20Check
  ;[0.3934 1 0] Check for Terrain Trail and Foliage Trample Volumes
  (bind _outactors (Collision|BoxOverlapActors (Transformation|GetActorLocation (Game|Player|GetPlayerPawn 0)) "1.000000,1.000000,1.000000" (Utilities|Array|MakeArray "ObjectTypeQuery2") 0 :!class /Script/Engine.KismetSystemLibrary))
  (for _array_element _outactors
    (Utilities|FlowControl|Sequence
      (:then_0
        (if (and (Variables|Activation|GetTerrain%20Trail%20System%20Activated) (== (Utilities|GetClass _array_element) "/Game/M4/Blueprints/SystemResources/Trails/EnablingVolumes/TerrainTrailVolume.TerrainTrailVolume_C"))
          (Utilities|FlowControl|Sequence
            (:then_0
              (Utilities|FlowControl|DoOnce false :!label _label
                (:Completed
                  (Variables|Default|SetTerrain%20Trail%20System%20Allowed true))))
            (:then_1
              (Utilities|FlowControl|RetriggerableDelay 4.0)
              (Variables|Default|SetTerrain%20Trail%20System%20Allowed false)
              (CallFunction|ClearTerrainTrailRenderTargets)
              (goto _label Reset)))))
      (:then_1
        (if (and (== (Utilities|GetClass _array_element) "/Game/M4/Blueprints/SystemResources/Trails/EnablingVolumes/FoliageTrampleVolume.FoliageTrampleVolume_C") (Variables|Activation|GetFoliage%20Trail%20System%20Activated))
          (Utilities|FlowControl|Sequence
            (:then_0
              (Utilities|FlowControl|DoOnce false :!label _label_2
                (:Completed
                  (Variables|Default|SetFoliage%20Trail%20System%20Allowed true)
                  (Variables|Default|SetLoop%20Detect%20Direction%20of%20Travel true)
                  (CallFunction|StartDirectionOfTravelDetection)
                  ;[0.3934 1 0] Forces Render Target Updating - for things like Grass Trampling fade out over time
                  (bind _returnvalue (Utilities|Time|SetTimerbyEvent (delegate Custom|Force%20Update) 0.1 (Variables|Default|GetLoop%20Detect%20Direction%20of%20Travel))))))
            (:then_1
              (Utilities|FlowControl|RetriggerableDelay 4.0)
              (Variables|Default|SetFoliage%20Trail%20System%20Allowed false)
              (Variables|Default|SetLoop%20Detect%20Direction%20of%20Travel false)
              (CallFunction|ClearFoliageTrailRenderTargets)
              (Utilities|Time|ClearandInvalidateTimerbyHandle _returnvalue)
              (goto _label_2 Reset))))))))

(event Custom|Start%20Checking%20for%20Trail%20Enable%20Overlaps
  ;[0.3934 1 0] Check for Terrain Trail and Foliage Trample Volumes
  (Utilities|Time|SetTimerbyEvent (delegate Custom|Volume%20Overlap%20Check) (Variables|Default|GetTrail%20and%20Trample%20Volume%20Check%20Tick) true))

(event Custom|Retry%20Terrain%20Trail
  (bind _returnvalue (Transformation|GetActorLocation))
  (bind _returnvalue_2 (/ 1.0 1024.0))
  (bind _returnvalue_3 (Transformation|GetActorLocation))
  (bind _returnvalue_4 (Game|Player|GetPlayerPawn 0))
  (bind _trail_area_of_effect (Variables|AreaSizes|GetTrail%20Area%20of%20Effect))
  (bind _trail_collider_array___last_record (Variables|Default|GetTrail%20Collider%20Array%20-%20Last%20Record))
  (bind _returnvalue_5 (Math|Conversions|ToLinearColor(Vector) _returnvalue))
  (bind _returnvalue_6 (Transformation|GetActorLocation _returnvalue_4))
  (bind _returnvalue_7 (* _trail_area_of_effect _returnvalue_2))
  (bind _return_value (Utilities|SnapPixeltoWorldGrid (.x _returnvalue_6) _returnvalue_7 (.y _returnvalue_6)))
  (bind _returnvalue_8 (- _return_value _returnvalue_3))
  ;[1 1 1] Trail Capturing
  (if (Utilities|Operators|EqualEqual (Utilities|Array|Get(acopy) (Variables|ColliderInformation|GetTrail%20Collider%20Location%20Array) (Variables|Default|GetIndex%20to%20Fetch)) (Utilities|Array|Get(acopy) _trail_collider_array___last_record (Variables|Default|GetIndex%20to%20Fetch)) (Variables|Default|GetDistance%20Between%20New%20Draw%20Locations))
    (CallFunction|GoThroughandCheckColliders(TerrainTrails))
    (else
      (Utilities|Array|SetArrayElem _trail_collider_array___last_record (Variables|Default|GetIndex%20to%20Fetch) (Utilities|Array|Get(acopy) (Variables|ColliderInformation|GetTrail%20Collider%20Location%20Array) (Variables|Default|GetIndex%20to%20Fetch)))
      (Rendering|Material|SetVectorParameterValue "/Game/M4/Blueprints/SystemResources/MagicMapMaterialBP/MPCs/PTM-MPC-Variables.PTM-MPC-Variables" "TrailTempAlphaOffset" (Math|Conversions|ToLinearColor(Vector) (- (Transformation|GetActorLocation (Game|Player|GetPlayerPawn 0)) (Utilities|Array|Get(acopy) (Variables|ColliderInformation|GetTrail%20Collider%20Location%20Array) (Variables|Default|GetIndex%20to%20Fetch)))) :!class /Script/Engine.KismetMaterialLibrary)
      (Rendering|Material|SetScalarParameterValue "/Game/M4/Blueprints/SystemResources/MagicMapMaterialBP/MPCs/PTM-MPC-Variables.PTM-MPC-Variables" "TrailStampSize" (Utilities|Array|Get(acopy) (Variables|ColliderInformation|GetTrail%20Collider%20Size%20Array) (Variables|Default|GetIndex%20to%20Fetch)) :!class /Script/Engine.KismetMaterialLibrary)
      (Utilities|FlowControl|Sequence
        (:then_0
          ;;[0.2475 0.4948 0.2345] Render Target - Temporary (Movement)
          (Variables|Default|SetTerrain%20Trails%20Move%20Offset (Math|Vector2D|MakeVector2D (.x _returnvalue_8) (.y _returnvalue_8)))
          (Transformation|AddActorWorldOffset (Math|Vector|MakeVector (.x _returnvalue_8) (.y _returnvalue_8) 0.0))
          (Rendering|Material|SetVectorParameterValue "/Game/M4/Blueprints/SystemResources/MagicMapMaterialBP/MPCs/PTM-MPC-Variables.PTM-MPC-Variables" "TrailCaptureLocation" _returnvalue_5 :!class /Script/Engine.KismetMaterialLibrary)
          (Rendering|Material|SetVectorParameterValue "/Game/M4/Blueprints/SystemResources/MagicMapMaterialBP/MPCs/PTM-MPC-Variables.PTM-MPC-Variables" "TrampleCaptureLocation" _returnvalue_5 :!class /Script/Engine.KismetMaterialLibrary)
          (Rendering|Material|SetVectorParameterValue "/Game/M4/Blueprints/SystemResources/MagicMapMaterialBP/MPCs/PTM-MPC-Variables.PTM-MPC-Variables" "Player Location" (Math|Conversions|ToLinearColor(Vector) (Transformation|GetActorLocation (Game|Player|GetPlayerPawn 0))) :!class /Script/Engine.KismetMaterialLibrary))
        (:then_1
          (Rendering|Material|SetVectorParameterValue "/Game/M4/Blueprints/SystemResources/MagicMapMaterialBP/MPCs/PTM-MPC-Variables.PTM-MPC-Variables" "TerrainTrailMoveOffset" (Utilities|Struct|MakeLinearColor (.x (/ (Variables|Default|GetTerrain%20Trails%20Move%20Offset) (Variables|AreaSizes|GetTrail%20Area%20of%20Effect))) (.y (/ (Variables|Default|GetTerrain%20Trails%20Move%20Offset) (Variables|AreaSizes|GetTrail%20Area%20of%20Effect))) 0.0 1.0) :!class /Script/Engine.KismetMaterialLibrary)
          (bind _output_get (Variables|Default|SetTerrain%20Trails%20Total%20Move%20Offset (Math|Vector2D|MakeVector2D (+ (.x (/ (Variables|Default|GetTerrain%20Trails%20Move%20Offset) (Variables|AreaSizes|GetTrail%20Area%20of%20Effect))) (.x (Variables|Default|GetTerrain%20Trails%20Total%20Move%20Offset))) (+ (.y (/ (Variables|Default|GetTerrain%20Trails%20Move%20Offset) (Variables|AreaSizes|GetTrail%20Area%20of%20Effect))) (.y (Variables|Default|GetTerrain%20Trails%20Total%20Move%20Offset))))))
          (Rendering|Material|SetVectorParameterValue "/Game/M4/Blueprints/SystemResources/MagicMapMaterialBP/MPCs/PTM-MPC-Variables.PTM-MPC-Variables" "TerrainTrailTotalOffset" (Utilities|Struct|MakeLinearColor (.x _output_get) (.y _output_get) 0.0 1.0) :!class /Script/Engine.KismetMaterialLibrary))
        (:then_2
          (Utilities|FlowControl|Sequence
            (:then_0
              (if (Variables|Default|GetTerrain%20Trail%20System%20Allowed)
                ;;[1 1 1] Writing Process for Terrain Trails
                (Rendering|DrawMaterialtoRenderTarget (Variables|RenderTargets|TerrainTrails|GetRT%20-%20Temporary%20-%20Terrain%20Trails) "/Game/M4/Blueprints/SystemResources/Trails/Materials/V3/Terrain/RT_TempMat_Inst.RT_TempMat_Inst")
                (Rendering|DrawMaterialtoRenderTarget (Variables|RenderTargets|TerrainTrails|GetRT%20-%20Persistent%20-%20Terrain%20Trails) "/Game/M4/Blueprints/SystemResources/Trails/Materials/V3/Terrain/RT_PersistentMat_Inst.RT_PersistentMat_Inst")
                (Rendering|DrawMaterialtoRenderTarget (Variables|RenderTargets|TerrainTrails|GetRT%20-%20Persistent%20Blurred%20-%20Terrain%20Trails) "/Game/M4/Blueprints/SystemResources/Trails/Materials/V3/Terrain/RT_BlurringMat_Inst.RT_BlurringMat_Inst")
                (Rendering|DrawMaterialtoRenderTarget (Variables|RenderTargets|TerrainTrails|GetRT%20-%20Persistent%20Normals%20-%20Terrain%20Trails) "/Game/M4/Blueprints/SystemResources/Trails/Materials/V3/Terrain/RT_NormalsMat_Inst.RT_NormalsMat_Inst")))
            (:then_1
              (if (Variables|Default|GetFoliage%20Trail%20System%20Allowed)
                ;;[1 1 1] Writing Process for Foliage Interaction
                (Rendering|DrawMaterialtoRenderTarget (Variables|RenderTargets|FoliageInteraction|GetRT%20-%20Temporary%20-%20Foliage%20Push) "/Game/M4/Blueprints/SystemResources/Trails/Materials/V3/Foliage/RT_FoliageTempMat_Inst.RT_FoliageTempMat_Inst")
                (Rendering|DrawMaterialtoRenderTarget (Variables|RenderTargets|FoliageInteraction|GetRT%20-%20Persistent%20-%20Foliage%20Push) "/Game/M4/Blueprints/SystemResources/Trails/Materials/V3/Foliage/RT_FoliagePersistentMat_Inst.RT_FoliagePersistentMat_Inst")
                (Rendering|DrawMaterialtoRenderTarget (Variables|RenderTargets|FoliageInteraction|GetRT%20-%20Persistent%20Blurred%20-%20Foliage%20Push) "/Game/M4/Blueprints/SystemResources/Trails/Materials/V3/Foliage/RT_FoliageBlurringMat_Inst.RT_FoliageBlurringMat_Inst")))))
        (:then_4
          (if (<= (- (Utilities|Array|Length (Variables|ColliderInformation|GetTrail%20Collider%20Location%20Array)) 1) (Variables|Default|GetIndex%20to%20Fetch))
            (Variables|Default|SetIndex%20to%20Fetch 0)
            (else
              (Variables|Default|SetIndex%20to%20Fetch (+ (Variables|Default|GetIndex%20to%20Fetch) 1))))
          (Variables|Default|SetOpen%20Capture%20Location true))))))

(event Custom|Start%20Direction%20of%20Travel%20Detection
  ;[0.0205 0.4638 1] Direction of Travel Detection
  (Utilities|Time|SetTimerbyEvent (delegate Custom|Set%20Direction%20of%20Travel) (Variables|Default|GetFoliage%20Bend%20Direction%20Detection%20Tick) (Variables|Default|GetLoop%20Detect%20Direction%20of%20Travel)))

(event Custom|Bypass%20Movement%20Check
  ;[1 1 1] Trail Capturing
)

(event Custom|Force%20Update
  (bind _trail_collider_array___last_record (Variables|Default|GetTrail%20Collider%20Array%20-%20Last%20Record))
  (bind _output (Utilities|Array|Get(acopy) _trail_collider_array___last_record))
  (bind _output_2 (Utilities|Array|Get(acopy) _trail_collider_array___last_record))
  ;[0.3934 1 0] Forces Render Target Updating - for things like Grass Trampling fade out over time
  (Utilities|FlowControl|FlipFlop
    (:A
      (Utilities|Array|SetArrayElem _trail_collider_array___last_record 0 (Math|Vector|MakeVector (.x _output_2) (.y _output_2) (+ (.z _output_2) 1e+01))))
    (:B
      (Utilities|Array|SetArrayElem _trail_collider_array___last_record 0 (Math|Vector|MakeVector (.x _output) (.y _output) (- (.z _output) 1e+01))))))

(event EventBeginPlay
  (bind _trail_area_of_effect (Variables|AreaSizes|GetTrail%20Area%20of%20Effect))
  (Utilities|FlowControl|Delay 0.5)
  (CallFunction|SetVariablesfromTrailandTrampleBP)
  (Rendering|Material|SetScalarParameterValue "/Game/M4/Blueprints/SystemResources/MagicMapMaterialBP/MPCs/PTM-MPC-Variables.PTM-MPC-Variables" "TrampleTexSize" _trail_area_of_effect :!class /Script/Engine.KismetMaterialLibrary)
  (Rendering|Material|SetScalarParameterValue "/Game/M4/Blueprints/SystemResources/MagicMapMaterialBP/MPCs/PTM-MPC-Variables.PTM-MPC-Variables" "TrailEffectSize" _trail_area_of_effect :!class /Script/Engine.KismetMaterialLibrary)
  (Variables|RenderTargets|TerrainTrails|SetRT%20-%20Temporary%20-%20Terrain%20Trails "/Game/M4/Blueprints/SystemResources/Trails/Textures/RTs/V3/TerrainTrails/RT_Trails_Temporary.RT_Trails_Temporary")
  (Variables|RenderTargets|TerrainTrails|SetRT%20-%20Persistent%20-%20Terrain%20Trails "/Game/M4/Blueprints/SystemResources/Trails/Textures/RTs/V3/TerrainTrails/RT_Trails_Persistent.RT_Trails_Persistent")
  (CallFunction|ClearFoliageTrailRenderTargets)
  (CallFunction|ClearTerrainTrailRenderTargets)
  (Utilities|FlowControl|Delay 0.2)
  (Variables|Default|SetTrail%20Collider%20Array%20-%20Last%20Record (Variables|ColliderInformation|GetTrail%20Collider%20Location%20Array))
  (CallFunction|StartCheckingforTrailEnableOverlaps))

(event Collision|EventActorBeginOverlap
  (params (OtherActor :type Actor%20Object%20Reference)))

(event EventTick
  (params (DeltaSeconds :type Float%20%28single-precision%29))
  (bind _returnvalue (Transformation|GetActorLocation))
  (bind _returnvalue_2 (/ 1.0 1024.0))
  (bind _returnvalue_3 (Transformation|GetActorLocation))
  (bind _returnvalue_4 (Game|Player|GetPlayerPawn 0))
  (bind _trail_area_of_effect (Variables|AreaSizes|GetTrail%20Area%20of%20Effect))
  (bind _returnvalue_5 (Math|Conversions|ToLinearColor(Vector) _returnvalue))
  (bind _returnvalue_6 (Transformation|GetActorLocation _returnvalue_4))
  (bind _returnvalue_7 (* _trail_area_of_effect _returnvalue_2))
  (bind _return_value (Utilities|SnapPixeltoWorldGrid (.x _returnvalue_6) _returnvalue_7 (.y _returnvalue_6)))
  (bind _returnvalue_8 (- _return_value _returnvalue_3))
  ;[1 1 1] Trail Capturing
  (if (or (Variables|Default|GetTerrain%20Trail%20System%20Allowed) (Variables|Default|GetFoliage%20Trail%20System%20Allowed))
    (if (== (Utilities|Array|Length (Variables|ColliderInformation|GetTrail%20Collider%20Location%20Array)) (Utilities|Array|Length (Variables|Default|GetTrail%20Collider%20Array%20-%20Last%20Record)))
      _
      (else
        (Variables|Default|SetTrail%20Collider%20Array%20-%20Last%20Record (Variables|ColliderInformation|GetTrail%20Collider%20Location%20Array))))
    (for _index (range 0 (Variables|Default|GetTrail%20Check%20Iteration%20Amount))
      (if (Utilities|Operators|EqualEqual (Utilities|Array|Get(acopy) (Variables|ColliderInformation|GetTrail%20Collider%20Location%20Array) (Variables|Default|GetIndex%20to%20Fetch)) (Utilities|Array|Get(acopy) (Variables|Default|GetTrail%20Collider%20Array%20-%20Last%20Record) (Variables|Default|GetIndex%20to%20Fetch)) (Variables|Default|GetDistance%20Between%20New%20Draw%20Locations))
        (CallFunction|GoThroughandCheckColliders(TerrainTrails))
        (else
          (Utilities|Array|SetArrayElem (Variables|Default|GetTrail%20Collider%20Array%20-%20Last%20Record) (Variables|Default|GetIndex%20to%20Fetch) (Utilities|Array|Get(acopy) (Variables|ColliderInformation|GetTrail%20Collider%20Location%20Array) (Variables|Default|GetIndex%20to%20Fetch)))
          (Rendering|Material|SetVectorParameterValue "/Game/M4/Blueprints/SystemResources/MagicMapMaterialBP/MPCs/PTM-MPC-Variables.PTM-MPC-Variables" "TrailTempAlphaOffset" (Math|Conversions|ToLinearColor(Vector) (- (Transformation|GetActorLocation (Game|Player|GetPlayerPawn 0)) (Utilities|Array|Get(acopy) (Variables|ColliderInformation|GetTrail%20Collider%20Location%20Array) (Variables|Default|GetIndex%20to%20Fetch)))) :!class /Script/Engine.KismetMaterialLibrary)
          (Rendering|Material|SetScalarParameterValue "/Game/M4/Blueprints/SystemResources/MagicMapMaterialBP/MPCs/PTM-MPC-Variables.PTM-MPC-Variables" "TrailStampSize" (Utilities|Array|Get(acopy) (Variables|ColliderInformation|GetTrail%20Collider%20Size%20Array) (Variables|Default|GetIndex%20to%20Fetch)) :!class /Script/Engine.KismetMaterialLibrary)
          (Utilities|FlowControl|Sequence
            (:then_0
              ;;[0.2475 0.4948 0.2345] Render Target - Temporary (Movement)
              (Variables|Default|SetTerrain%20Trails%20Move%20Offset (Math|Vector2D|MakeVector2D (.x _returnvalue_8) (.y _returnvalue_8)))
              (Transformation|AddActorWorldOffset (Math|Vector|MakeVector (.x _returnvalue_8) (.y _returnvalue_8) 0.0))
              (Rendering|Material|SetVectorParameterValue "/Game/M4/Blueprints/SystemResources/MagicMapMaterialBP/MPCs/PTM-MPC-Variables.PTM-MPC-Variables" "TrailCaptureLocation" _returnvalue_5 :!class /Script/Engine.KismetMaterialLibrary)
              (Rendering|Material|SetVectorParameterValue "/Game/M4/Blueprints/SystemResources/MagicMapMaterialBP/MPCs/PTM-MPC-Variables.PTM-MPC-Variables" "TrampleCaptureLocation" _returnvalue_5 :!class /Script/Engine.KismetMaterialLibrary)
              (Rendering|Material|SetVectorParameterValue "/Game/M4/Blueprints/SystemResources/MagicMapMaterialBP/MPCs/PTM-MPC-Variables.PTM-MPC-Variables" "Player Location" (Math|Conversions|ToLinearColor(Vector) (Transformation|GetActorLocation (Game|Player|GetPlayerPawn 0))) :!class /Script/Engine.KismetMaterialLibrary))
            (:then_1
              (Rendering|Material|SetVectorParameterValue "/Game/M4/Blueprints/SystemResources/MagicMapMaterialBP/MPCs/PTM-MPC-Variables.PTM-MPC-Variables" "TerrainTrailMoveOffset" (Utilities|Struct|MakeLinearColor (.x (/ (Variables|Default|GetTerrain%20Trails%20Move%20Offset) (Variables|AreaSizes|GetTrail%20Area%20of%20Effect))) (.y (/ (Variables|Default|GetTerrain%20Trails%20Move%20Offset) (Variables|AreaSizes|GetTrail%20Area%20of%20Effect))) 0.0 1.0) :!class /Script/Engine.KismetMaterialLibrary)
              (bind _output_get (Variables|Default|SetTerrain%20Trails%20Total%20Move%20Offset (Math|Vector2D|MakeVector2D (+ (.x (/ (Variables|Default|GetTerrain%20Trails%20Move%20Offset) (Variables|AreaSizes|GetTrail%20Area%20of%20Effect))) (.x (Variables|Default|GetTerrain%20Trails%20Total%20Move%20Offset))) (+ (.y (/ (Variables|Default|GetTerrain%20Trails%20Move%20Offset) (Variables|AreaSizes|GetTrail%20Area%20of%20Effect))) (.y (Variables|Default|GetTerrain%20Trails%20Total%20Move%20Offset))))))
              (Rendering|Material|SetVectorParameterValue "/Game/M4/Blueprints/SystemResources/MagicMapMaterialBP/MPCs/PTM-MPC-Variables.PTM-MPC-Variables" "TerrainTrailTotalOffset" (Utilities|Struct|MakeLinearColor (.x _output_get) (.y _output_get) 0.0 1.0) :!class /Script/Engine.KismetMaterialLibrary))
            (:then_2
              (Utilities|FlowControl|Sequence
                (:then_0
                  (if (Variables|Default|GetTerrain%20Trail%20System%20Allowed)
                    ;;[1 1 1] Writing Process for Terrain Trails
                    (Rendering|DrawMaterialtoRenderTarget (Variables|RenderTargets|TerrainTrails|GetRT%20-%20Temporary%20-%20Terrain%20Trails) "/Game/M4/Blueprints/SystemResources/Trails/Materials/V3/Terrain/RT_TempMat_Inst.RT_TempMat_Inst")
                    (Rendering|DrawMaterialtoRenderTarget (Variables|RenderTargets|TerrainTrails|GetRT%20-%20Persistent%20-%20Terrain%20Trails) "/Game/M4/Blueprints/SystemResources/Trails/Materials/V3/Terrain/RT_PersistentMat_Inst.RT_PersistentMat_Inst")
                    (Rendering|DrawMaterialtoRenderTarget (Variables|RenderTargets|TerrainTrails|GetRT%20-%20Persistent%20Blurred%20-%20Terrain%20Trails) "/Game/M4/Blueprints/SystemResources/Trails/Materials/V3/Terrain/RT_BlurringMat_Inst.RT_BlurringMat_Inst")
                    (Rendering|DrawMaterialtoRenderTarget (Variables|RenderTargets|TerrainTrails|GetRT%20-%20Persistent%20Normals%20-%20Terrain%20Trails) "/Game/M4/Blueprints/SystemResources/Trails/Materials/V3/Terrain/RT_NormalsMat_Inst.RT_NormalsMat_Inst")))
                (:then_1
                  (if (Variables|Default|GetFoliage%20Trail%20System%20Allowed)
                    ;;[1 1 1] Writing Process for Foliage Interaction
                    (Rendering|DrawMaterialtoRenderTarget (Variables|RenderTargets|FoliageInteraction|GetRT%20-%20Temporary%20-%20Foliage%20Push) "/Game/M4/Blueprints/SystemResources/Trails/Materials/V3/Foliage/RT_FoliageTempMat_Inst.RT_FoliageTempMat_Inst")
                    (Rendering|DrawMaterialtoRenderTarget (Variables|RenderTargets|FoliageInteraction|GetRT%20-%20Persistent%20-%20Foliage%20Push) "/Game/M4/Blueprints/SystemResources/Trails/Materials/V3/Foliage/RT_FoliagePersistentMat_Inst.RT_FoliagePersistentMat_Inst")
                    (Rendering|DrawMaterialtoRenderTarget (Variables|RenderTargets|FoliageInteraction|GetRT%20-%20Persistent%20Blurred%20-%20Foliage%20Push) "/Game/M4/Blueprints/SystemResources/Trails/Materials/V3/Foliage/RT_FoliageBlurringMat_Inst.RT_FoliageBlurringMat_Inst")))))
            (:then_4
              (if (<= (- (Utilities|Array|Length (Variables|ColliderInformation|GetTrail%20Collider%20Location%20Array)) 1) (Variables|Default|GetIndex%20to%20Fetch))
                (Variables|Default|SetIndex%20to%20Fetch 0)
                (else
                  (Variables|Default|SetIndex%20to%20Fetch (+ (Variables|Default|GetIndex%20to%20Fetch) 1))))
              (Variables|Default|SetOpen%20Capture%20Location true))))))))

(fn ConstructionScript)

(fn SetVariablesfromTrailandTrampleBP
  (bind _returnvalue (Actor|GetActorOfClass "/Game/M4/Blueprints/TrailsAndTrampleBP.TrailsAndTrampleBP_C"))
  (Utilities|IsValid _returnvalue
    (:Is%20Valid
      (Variables|Default|SetTrail%20Check%20Iteration%20Amount (- (Variables|/Game/M4/Blueprints/TrailsAndTrampleBP.TrailsAndTrampleBP_C|GetTrail%20Check%20Iterations%20%28Read%20Tooltip%29 _returnvalue) 1))
      (switch Utilities|FlowControl|Switch|SwitchonTrailCaptureSize (Variables|/Game/M4/Blueprints/TrailsAndTrampleBP.TrailsAndTrampleBP_C|GetTrail%20Capture%20Size%20%28Effects%20Quality%20&%20Capture%20Distance%29%20[Experimental] _returnvalue)
        (:NewEnumerator3
          (Variables|AreaSizes|SetTrail%20Area%20of%20Effect 4096.0))
        (:NewEnumerator0
          (Variables|AreaSizes|SetTrail%20Area%20of%20Effect 8192.0))
        (:NewEnumerator1
          (Variables|AreaSizes|SetTrail%20Area%20of%20Effect 16384.0)))
      (Variables|Activation|SetFoliage%20Trail%20System%20Activated (Variables|/Game/M4/Blueprints/TrailsAndTrampleBP.TrailsAndTrampleBP_C|GetEnable%20Foliage%20Interaction%20System%20%28Read%20Tooltip%29 _returnvalue))
      (Variables|Activation|SetTerrain%20Trail%20System%20Activated (Variables|/Game/M4/Blueprints/TrailsAndTrampleBP.TrailsAndTrampleBP_C|GetEnable%20Terrain%20Trail%20System%20%28Read%20Tooltip%29 _returnvalue)))
    (:Is%20Not%20Valid
      _))
  (return))

(fn GoThroughandCheckColliders(TerrainTrails)
  (bind _trail_collider_location_array (Variables|ColliderInformation|GetTrail%20Collider%20Location%20Array))
  (bind _returnvalue (Utilities|Array|Length _trail_collider_location_array))
  (bind _returnvalue_2 (- _returnvalue 1))
  (if (<= _returnvalue_2 (Variables|Default|GetIndex%20to%20Fetch))
    (Variables|Default|SetIndex%20to%20Fetch 0)
    (else
      (bind _index (Utilities|FlowControl|ForLoopwithBreak (Variables|Default|GetIndex%20to%20Fetch) _returnvalue_2 :!label _label)
        (:LoopBody
          (Variables|Default|SetIndex%20to%20Fetch _index)
          (if (not (Utilities|Operators|EqualEqual (Utilities|Array|Get(acopy) (Variables|ColliderInformation|GetTrail%20Collider%20Location%20Array) _index) (Utilities|Array|Get(acopy) (Variables|Default|GetTrail%20Collider%20Array%20-%20Last%20Record) _index) (Variables|Default|GetDistance%20Between%20New%20Draw%20Locations)))
            (CallFunction|RetryTerrainTrail)
            (goto _label Break)))))))

(fn ClearFoliageTrailRenderTargets
  (Rendering|ClearRenderTarget2D (Variables|RenderTargets|FoliageInteraction|GetRT%20-%20Temporary%20-%20Foliage%20Push))
  (Rendering|ClearRenderTarget2D (Variables|RenderTargets|FoliageInteraction|GetRT%20-%20Persistent%20-%20Foliage%20Push))
  (Rendering|ClearRenderTarget2D (Variables|RenderTargets|FoliageInteraction|GetRT%20-%20Persistent%20Blurred%20-%20Foliage%20Push)))

(fn ClearTerrainTrailRenderTargets
  (Rendering|ClearRenderTarget2D (Variables|RenderTargets|TerrainTrails|GetRT%20-%20Temporary%20-%20Terrain%20Trails))
  (Rendering|ClearRenderTarget2D (Variables|RenderTargets|TerrainTrails|GetRT%20-%20Persistent%20-%20Terrain%20Trails))
  (Rendering|ClearRenderTarget2D (Variables|RenderTargets|TerrainTrails|GetRT%20-%20Persistent%20Blurred%20-%20Terrain%20Trails))
  (Rendering|ClearRenderTarget2D (Variables|RenderTargets|TerrainTrails|GetRT%20-%20Persistent%20Normals%20-%20Terrain%20Trails)))