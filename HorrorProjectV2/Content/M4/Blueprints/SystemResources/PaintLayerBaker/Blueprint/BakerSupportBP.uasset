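; BakerSupportBP is an editor-time helper actor that bakes terrain paint layer splatmaps for biome presets.
; BakeOut clears the baked splat render target and triggers a scene capture.
; Upscale&Blur draws an upscale-and-blur material into a finalized render target, then converts it to the Island, Tundra or Desert splatmap texture via an editor-only conversion.
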(event Custom|Bake%20Out
  (params (Selected%20Terrain%20Biome%20Preset :type TerrainBiomePresets%20Enum :default "NewEnumerator0") (Selected%20Terrain%20Performance%20Preset :type PerformancePreferences%20Enum :default "NewEnumerator7"))
  (Rendering|ClearRenderTarget2D (Variables|Default|GetBakedSplatRT))
  (Rendering|SceneCapture|CaptureScene (Variables|Default|GetSceneCaptureComponent2D) :!class /Script/Engine.SceneCaptureComponent2D))

(event Custom|Upscale%20&%20Blur
  (params (Selected%20Terrain%20Biome%20Preset :type TerrainBiomePresets%20Enum :default "NewEnumerator0"))
  (Rendering|ClearRenderTarget2D "/Game/M4/Blueprints/SystemResources/RenderTargets/SplatBaker/SplatmapPrework/FinalizedSplatMapRT.FinalizedSplatMapRT")
  (Rendering|DrawMaterialtoRenderTarget "/Game/M4/Blueprints/SystemResources/RenderTargets/SplatBaker/SplatmapPrework/FinalizedSplatMapRT.FinalizedSplatMapRT" "/Game/M4/Blueprints/SystemResources/SplatBakerBP/Materials/UpscaleAndBlurMat_Inst.UpscaleAndBlurMat_Inst")
  (switch Utilities|FlowControl|Switch|SwitchonTerrainBiomePresets Selected%20Terrain%20Biome%20Preset
    (:NewEnumerator0
      (EditorScripting|Rendering|ConvertRenderTargettoTexture2DEditorOnly "/Game/M4/Blueprints/SystemResources/RenderTargets/SplatBaker/SplatmapPrework/FinalizedSplatMapRT.FinalizedSplatMapRT" "/Game/M4/Blueprints/SystemResources/RenderTargets/SplatBaker/IslandHM/IslandFinalizedSplatmap.IslandFinalizedSplatmap"))
    (:NewEnumerator1
      (EditorScripting|Rendering|ConvertRenderTargettoTexture2DEditorOnly "/Game/M4/Blueprints/SystemResources/RenderTargets/SplatBaker/SplatmapPrework/FinalizedSplatMapRT.FinalizedSplatMapRT" "/Game/M4/Blueprints/SystemResources/RenderTargets/SplatBaker/TundraHM/TundraFinalizedSplatmap.TundraFinalizedSplatmap"))
    (:NewEnumerator2
      (EditorScripting|Rendering|ConvertRenderTargettoTexture2DEditorOnly "/Game/M4/Blueprints/SystemResources/RenderTargets/SplatBaker/SplatmapPrework/FinalizedSplatMapRT.FinalizedSplatMapRT" "/Game/M4/Blueprints/SystemResources/RenderTargets/SplatBaker/DesertHM/DesertFinalizedSplatmap.DesertFinalizedSplatmap"))))

(event EventBeginPlay)

(event Collision|EventActorBeginOverlap
  (params (OtherActor :type Actor%20Object%20Reference)))

(event EventTick
  (params (DeltaSeconds :type Float%20%28single-precision%29)))

(fn ConstructionScript)