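; Virtual heightfield actor that renders displaced landscape from height and color runtime virtual textures, using a Niagara grid of tiled plane meshes.
; Its construction script configures tile grid, LOD distances, per-LOD mesh density and shadows, or hides the system when disabled.
; Dynamic materials receive the RVTs, with optional per-LOD debug materials.
; After a BeginPlay delay, it invalidates large RVT volumes around the player (or origin) and small ones around origin.
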(event Custom|Setup%20M4%20Custom%20Displacement
  (bind _tesssystem (Variables|Default|GetTessSystem))
  (if (Variables|Visuals|GetEnable%20System)
    (Rendering|SetVisibility _tesssystem true false)
    (Niagara|SetNiagaraVariable(Float) _tesssystem "GridSpacing" (Variables|LevelOfDetail|LODSections|GetLOD%20Tile%20Size))
    (Class|NiagaraComponent|SetVariableInt _tesssystem "MaxNumTilesAcross" (Variables|LevelOfDetail|LODSections|GetNumber%20of%20Tiles))
    (Niagara|SetNiagaraVariable(Float) _tesssystem "LOD0_MaxDistance" (Variables|LevelOfDetail|LODDistances|GetLOD%200%20Max%20Distance))
    (Niagara|SetNiagaraVariable(Float) _tesssystem "LOD1_MaxDistance" (Variables|LevelOfDetail|LODDistances|GetLOD%201%20Max%20Distance))
    (Niagara|SetNiagaraVariable(Float) _tesssystem "LOD2_MaxDistance" (Variables|LevelOfDetail|LODDistances|GetLOD%202%20Max%20Distance))
    (Rendering|SetCastShadow _tesssystem (Variables|Visuals|GetCast%20Shadows%20from%20Displacement))
    (Utilities|FlowControl|Sequence
      (:then_0
        (Utilities|FlowControl|Sequence
          (:then_0
            (Utilities|IsValid (Variables|AutoCaching|GetLandscape_Heightfield_MID)
              (:Is%20Not%20Valid
                (bind _returnvalue (Rendering|Material|CreateDynamicMaterialInstance (Variables|Visuals|GetHeightfield%20Material) "None" "None" :!class /Script/Engine.KismetMaterialLibrary))
                (Variables|AutoCaching|SetLandscape_Heightfield_MID _returnvalue))))
          (:then_1
            (Utilities|IsValid (Variables|AutoCaching|GetLOD0_Debug_MID)
              (:Is%20Not%20Valid
                (bind _returnvalue_2 (Rendering|Material|CreateDynamicMaterialInstance "/Game/M4/Blueprints/SystemResources/Heightfield/Materials/Debug/LOD0_DebugMat_Inst.LOD0_DebugMat_Inst" "None" "None" :!class /Script/Engine.KismetMaterialLibrary))
                (Variables|AutoCaching|SetLOD0_Debug_MID _returnvalue_2)
                (Class|MaterialInstanceDynamic|SetRuntimeVirtualTextureParameterValue (Variables|AutoCaching|GetLOD0_Debug_MID) "HeightRVT" (Variables|RuntimeVirtualTexturestoUse|GetHeight%20RVT)))))
          (:then_2
            (Utilities|IsValid (Variables|AutoCaching|GetLOD1_Debug_MID)
              (:Is%20Not%20Valid
                (bind _returnvalue_3 (Rendering|Material|CreateDynamicMaterialInstance "/Game/M4/Blueprints/SystemResources/Heightfield/Materials/Debug/LOD1_DebugMat_Inst.LOD1_DebugMat_Inst" "None" "None" :!class /Script/Engine.KismetMaterialLibrary))
                (Variables|AutoCaching|SetLOD1_Debug_MID _returnvalue_3)
                (Class|MaterialInstanceDynamic|SetRuntimeVirtualTextureParameterValue (Variables|AutoCaching|GetLOD1_Debug_MID) "HeightRVT" (Variables|RuntimeVirtualTexturestoUse|GetHeight%20RVT)))))
          (:then_3
            (Utilities|IsValid (Variables|AutoCaching|GetLOD2_Debug_MID)
              (:Is%20Not%20Valid
                (bind _returnvalue_4 (Rendering|Material|CreateDynamicMaterialInstance "/Game/M4/Blueprints/SystemResources/Heightfield/Materials/Debug/LOD2_DebugMat_Inst.LOD2_DebugMat_Inst" "None" "None" :!class /Script/Engine.KismetMaterialLibrary))
                (Variables|AutoCaching|SetLOD2_Debug_MID _returnvalue_4)
                (Class|MaterialInstanceDynamic|SetRuntimeVirtualTextureParameterValue (Variables|AutoCaching|GetLOD2_Debug_MID) "HeightRVT" (Variables|RuntimeVirtualTexturestoUse|GetHeight%20RVT)))))))
      (:then_1
        (Class|MaterialInstanceDynamic|SetRuntimeVirtualTextureParameterValue (Variables|AutoCaching|GetLandscape_Heightfield_MID) "ColorRVT" (Variables|RuntimeVirtualTexturestoUse|GetColor%20RVT))
        (Class|MaterialInstanceDynamic|SetRuntimeVirtualTextureParameterValue (Variables|AutoCaching|GetLandscape_Heightfield_MID) "HeightRVT" (Variables|RuntimeVirtualTexturestoUse|GetHeight%20RVT)))
      (:then_2
        (if (Variables|LevelOfDetail|GetShow%20LOD%20Debug)
          (Class|NiagaraComponent|SetVariableMaterial _tesssystem "LOD0_Material" (Variables|AutoCaching|GetLOD0_Debug_MID))
          (Class|NiagaraComponent|SetVariableMaterial _tesssystem "LOD1_Material" (Variables|AutoCaching|GetLOD1_Debug_MID))
          (Class|NiagaraComponent|SetVariableMaterial _tesssystem "LOD2_Material" (Variables|AutoCaching|GetLOD2_Debug_MID))
          (else
            (Class|NiagaraComponent|SetVariableMaterial _tesssystem "LOD0_Material" (Variables|AutoCaching|GetLandscape_Heightfield_MID))
            (Class|NiagaraComponent|SetVariableMaterial _tesssystem "LOD1_Material" (Variables|AutoCaching|GetLandscape_Heightfield_MID))
            (Class|NiagaraComponent|SetVariableMaterial _tesssystem "LOD2_Material" (Variables|AutoCaching|GetLandscape_Heightfield_MID)))))
      (:then_3
        (CallFunction|SetLODMeshes _tesssystem)))
    (else
      (Rendering|SetVisibility _tesssystem false false))))

(event EventBeginPlay
  (Utilities|FlowControl|Delay 2.0)
  (CallFunction|ResetHeightfieldAroundPlayer))

(event Collision|EventActorBeginOverlap
  (params (OtherActor :type Actor%20Object%20Reference)))

(event EventTick
  (params (DeltaSeconds :type Float%20%28single-precision%29)))

(fn ConstructionScript
  (CallFunction|SetupM4CustomDisplacement))

(fn ResetHeightfieldAroundPlayer
  (bind _returnvalue (Game|GetPlayerCharacter 0))
  (bind _returnvalue_2 (Transformation|GetActorLocation _returnvalue))
  (Utilities|IsValid (Game|GetPlayerCharacter 0)
    (:Is%20Valid
      (bind _returnvalue_3 (Actor|GetActorOfClass "/Game/M4/Blueprints/SystemResources/RVT/Volumes/RVT-Volume-Height-Large.RVT-Volume-Height-Large_C"))
      (Utilities|IsValid _returnvalue_3
        (:Is%20Valid
          (Class|RuntimeVirtualTextureComponent|Invalidate (Variables|/Script/Engine.RuntimeVirtualTextureVolume|GetVirtualTextureComponent _returnvalue_3) (Utilities|Struct|MakeBoxSphereBounds _returnvalue_2 (.BoxExtent (Collision|GetActorBounds _returnvalue_3 false false)) 2e+05)))
        (:Is%20Not%20Valid
          _))
      (bind _returnvalue_4 (Actor|GetActorOfClass "/Game/M4/Blueprints/SystemResources/RVT/Volumes/RVT-Volume-Color-Large.RVT-Volume-Color-Large_C"))
      (Utilities|IsValid _returnvalue_4
        (:Is%20Valid
          (Class|RuntimeVirtualTextureComponent|Invalidate (Variables|/Script/Engine.RuntimeVirtualTextureVolume|GetVirtualTextureComponent _returnvalue_4) (Utilities|Struct|MakeBoxSphereBounds _returnvalue_2 (.BoxExtent (Collision|GetActorBounds _returnvalue_3 false false)) 2e+05)))
        (:Is%20Not%20Valid
          _)))
    (:Is%20Not%20Valid
      (bind _returnvalue_5 (Actor|GetActorOfClass "/Game/M4/Blueprints/SystemResources/RVT/Volumes/RVT-Volume-Height-Large.RVT-Volume-Height-Large_C"))
      (Utilities|IsValid _returnvalue_5
        (:Is%20Valid
          (Class|RuntimeVirtualTextureComponent|Invalidate (Variables|/Script/Engine.RuntimeVirtualTextureVolume|GetVirtualTextureComponent _returnvalue_5) (Utilities|Struct|MakeBoxSphereBounds "0, 0, 0" (.BoxExtent (Collision|GetActorBounds _returnvalue_5 false false)) 5e+06)))
        (:Is%20Not%20Valid
          _))
      (bind _returnvalue_6 (Actor|GetActorOfClass "/Game/M4/Blueprints/SystemResources/RVT/Volumes/RVT-Volume-Color-Large.RVT-Volume-Color-Large_C"))
      (Utilities|IsValid _returnvalue_6
        (:Is%20Valid
          (Class|RuntimeVirtualTextureComponent|Invalidate (Variables|/Script/Engine.RuntimeVirtualTextureVolume|GetVirtualTextureComponent _returnvalue_6) (Utilities|Struct|MakeBoxSphereBounds "0, 0, 0" (.BoxExtent (Collision|GetActorBounds _returnvalue_5 false false)) 5e+06)))
        (:Is%20Not%20Valid
          _))))
  (bind _returnvalue_7 (Actor|GetActorOfClass "/Game/M4/Blueprints/SystemResources/RVT/Volumes/RVT-Volume-Height-Small.RVT-Volume-Height-Small_C"))
  (Utilities|IsValid _returnvalue_7
    (:Is%20Valid
      (Class|RuntimeVirtualTextureComponent|Invalidate (Variables|/Script/Engine.RuntimeVirtualTextureVolume|GetVirtualTextureComponent _returnvalue_7) (Utilities|Struct|MakeBoxSphereBounds "0, 0, 0" (.BoxExtent (Collision|GetActorBounds _returnvalue_7 false false)) 5e+05)))
    (:Is%20Not%20Valid
      _))
  (bind _returnvalue_8 (Actor|GetActorOfClass "/Game/M4/Blueprints/SystemResources/RVT/Volumes/RVT-Volume-Color-Small.RVT-Volume-Color-Small_C"))
  (Utilities|IsValid _returnvalue_8
    (:Is%20Valid
      (Class|RuntimeVirtualTextureComponent|Invalidate (Variables|/Script/Engine.RuntimeVirtualTextureVolume|GetVirtualTextureComponent _returnvalue_8) (Utilities|Struct|MakeBoxSphereBounds "0, 0, 0" (.BoxExtent (Collision|GetActorBounds _returnvalue_7 false false)) 5e+05)))
    (:Is%20Not%20Valid
      _))
  (return))

(fn SetLODMeshes
  (params (Niagara%20System :type Niagara%20Component%20Object%20Reference))
  (Utilities|FlowControl|Sequence
    (:then_0
      (switch Utilities|FlowControl|Switch|SwitchonHeightfieldLOD_Enum (Variables|LevelOfDetail|LODSections|GetLOD%200)
        (:NewEnumerator0
          (Class|NiagaraComponent|SetVariableStaticMesh Niagara%20System "LOD0_Mesh" "/Game/M4/Blueprints/SystemResources/Heightfield/Meshes/Plane_128Poly.Plane_128Poly"))
        (:NewEnumerator1
          (Class|NiagaraComponent|SetVariableStaticMesh Niagara%20System "LOD0_Mesh" "/Game/M4/Blueprints/SystemResources/Heightfield/Meshes/Plane_512Poly.Plane_512Poly"))
        (:NewEnumerator2
          (Class|NiagaraComponent|SetVariableStaticMesh Niagara%20System "LOD0_Mesh" "/Game/M4/Blueprints/SystemResources/Heightfield/Meshes/Plane_2kPoly.Plane_2kPoly"))
        (:NewEnumerator3
          (Class|NiagaraComponent|SetVariableStaticMesh Niagara%20System "LOD0_Mesh" "/Game/M4/Blueprints/SystemResources/Heightfield/Meshes/Plane_8kPoly.Plane_8kPoly"))
        (:NewEnumerator4
          (Class|NiagaraComponent|SetVariableStaticMesh Niagara%20System "LOD0_Mesh" "/Game/M4/Blueprints/SystemResources/Heightfield/Meshes/Plane_32kPoly.Plane_32kPoly"))))
    (:then_1
      (switch Utilities|FlowControl|Switch|SwitchonHeightfieldLOD_Enum (Variables|LevelOfDetail|LODSections|GetLOD%201)
        (:NewEnumerator0
          (Class|NiagaraComponent|SetVariableStaticMesh Niagara%20System "LOD1_Mesh" "/Game/M4/Blueprints/SystemResources/Heightfield/Meshes/Plane_128Poly.Plane_128Poly"))
        (:NewEnumerator1
          (Class|NiagaraComponent|SetVariableStaticMesh Niagara%20System "LOD1_Mesh" "/Game/M4/Blueprints/SystemResources/Heightfield/Meshes/Plane_512Poly.Plane_512Poly"))
        (:NewEnumerator2
          (Class|NiagaraComponent|SetVariableStaticMesh Niagara%20System "LOD1_Mesh" "/Game/M4/Blueprints/SystemResources/Heightfield/Meshes/Plane_2kPoly.Plane_2kPoly"))
        (:NewEnumerator3
          (Class|NiagaraComponent|SetVariableStaticMesh Niagara%20System "LOD1_Mesh" "/Game/M4/Blueprints/SystemResources/Heightfield/Meshes/Plane_8kPoly.Plane_8kPoly"))
        (:NewEnumerator4
          (Class|NiagaraComponent|SetVariableStaticMesh Niagara%20System "LOD1_Mesh" "/Game/M4/Blueprints/SystemResources/Heightfield/Meshes/Plane_32kPoly.Plane_32kPoly"))))
    (:then_2
      (switch Utilities|FlowControl|Switch|SwitchonHeightfieldLOD_Enum (Variables|LevelOfDetail|LODSections|GetLOD%202)
        (:NewEnumerator0
          (Class|NiagaraComponent|SetVariableStaticMesh Niagara%20System "LOD2_Mesh" "/Game/M4/Blueprints/SystemResources/Heightfield/Meshes/Plane_128Poly.Plane_128Poly"))
        (:NewEnumerator1
          (Class|NiagaraComponent|SetVariableStaticMesh Niagara%20System "LOD2_Mesh" "/Game/M4/Blueprints/SystemResources/Heightfield/Meshes/Plane_512Poly.Plane_512Poly"))
        (:NewEnumerator2
          (Class|NiagaraComponent|SetVariableStaticMesh Niagara%20System "LOD2_Mesh" "/Game/M4/Blueprints/SystemResources/Heightfield/Meshes/Plane_2kPoly.Plane_2kPoly"))
        (:NewEnumerator3
          (Class|NiagaraComponent|SetVariableStaticMesh Niagara%20System "LOD2_Mesh" "/Game/M4/Blueprints/SystemResources/Heightfield/Meshes/Plane_8kPoly.Plane_8kPoly"))
        (:NewEnumerator4
          (Class|NiagaraComponent|SetVariableStaticMesh Niagara%20System "LOD2_Mesh" "/Game/M4/Blueprints/SystemResources/Heightfield/Meshes/Plane_32kPoly.Plane_32kPoly"))))))