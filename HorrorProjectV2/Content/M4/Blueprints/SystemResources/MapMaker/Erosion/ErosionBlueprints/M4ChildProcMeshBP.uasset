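; M4 map maker erosion child actor that builds a grid procedural mesh, named as a scatter mesh.
; MakeScatterMesh sizes the grid from a landscape Blueprint's overall resolution and quad size, while MakeCustomScatterMesh uses its own vertex count and spacing variables.
; Both use CreateGridMeshSplit and replace mesh section 0 with the result, including two UV channels.
; Construction script and events are empty, so generation runs only when called.
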(event EventBeginPlay)

(event Collision|EventActorBeginOverlap
  (params (OtherActor :type Actor%20Object%20Reference)))

(event EventTick
  (params (DeltaSeconds :type Float%20%28single-precision%29)))

(fn ConstructionScript)

(fn MakeScatterMesh
  (params (LS%20BP :type Landmass%20Preview%20Mesh%20Object%20Reference))
  (bind _proceduralmesh (Variables|Default|GetProceduralMesh))
  (bind _output_get (Variables|Default|SetLS%20BP LS%20BP))
  (Utilities|IsValid _output_get
    (:Is%20Valid
      (bind (_triangles _vertices _uvs _uv1s) (Class|KismetProceduralMeshLibrary|CreateGridMeshSplit (Math|Float|Truncate (.X (Math|Vector2D|BreakVector2D (Variables|/Game/M4/Blueprints/LandmassPreviewMesh.LandmassPreviewMesh_C|GetOverall%20Resolution (Variables|Default|GetLS%20BP))))) (Math|Float|Truncate (.Y (Math|Vector2D|BreakVector2D (Variables|/Game/M4/Blueprints/LandmassPreviewMesh.LandmassPreviewMesh_C|GetOverall%20Resolution (Variables|Default|GetLS%20BP))))) (Variables|/Game/M4/Blueprints/LandmassPreviewMesh.LandmassPreviewMesh_C|GetSizePerQuad (Variables|Default|GetLS%20BP))))
      (Class|ProceduralMeshComponent|ClearMeshSection _proceduralmesh)
      (Class|ProceduralMeshComponent|CreateMeshSectionLinearColor _proceduralmesh 0 _vertices _triangles 0 _uvs _uv1s 0 0 0 0 false false))
    (:Is%20Not%20Valid
      (Development|PrintString "Invalid Landscape BP which should not be possible. "))))

(fn MakeCustomScatterMesh
  (bind _proceduralmesh (Variables|Default|GetProceduralMesh))
  (bind (_triangles _vertices _uvs _uv1s) (Class|KismetProceduralMeshLibrary|CreateGridMeshSplit (Variables|Custom|GetCustom%20Verts%20X) (Variables|Custom|GetCustom%20Verts%20Y) (Variables|Custom|GetCustom%20Quad%20Size)))
  (Class|ProceduralMeshComponent|ClearMeshSection _proceduralmesh)
  (Class|ProceduralMeshComponent|CreateMeshSectionLinearColor _proceduralmesh 0 _vertices _triangles 0 _uvs _uv1s 0 0 0 0 false false))