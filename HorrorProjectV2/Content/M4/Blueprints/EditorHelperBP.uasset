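; Editor helper actor that turns its exposed properties into rendering console commands for Lumen, virtual shadow maps, sharpening, screen percentage and anti-aliasing.
; The construction script and BeginPlay both run the four setter functions, and BeginPlay also destroys the logo and text components.
; Lumen and shadow map setters mirror their enable flags to WorldLightingBP, with shadows syncing only when the flag differs from the current console variable.
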(event EventBeginPlay
  (Lumen|SetLumen)
  (Extras|SetExtras)
  (VirtualShadowMaps|SetVirtualShadowMaps)
  (AntiAliasing|SetAnti-AliasingMode)
  (Components|DestroyComponent (Variables|Default|GetUnrealLogo)))

(event Collision|EventActorBeginOverlap
  (params (OtherActor :type Actor%20Object%20Reference)))

(event EventTick
  (params (DeltaSeconds :type Float%20%28single-precision%29)))

(fn ConstructionScript
  (Lumen|SetLumen)
  (Extras|SetExtras)
  (VirtualShadowMaps|SetVirtualShadowMaps)
  (AntiAliasing|SetAnti-AliasingMode))

(fn SetLumen
  (if (Variables|Lumen|GetEnable%20Lumen)
    (Development|ExecuteConsoleCommand "r.Lumen.DiffuseIndirect.Allow 1" 0)
    (Utilities|FlowControl|Sequence
      (:then_0
        (Utilities|FlowControl|Sequence
          (:then_0
            (if (not (== (Variables|Lumen|GetLumen%20Max%20Brightness) (Variables|TempSettings|GetLumen%20Max%20Brightness%20%28Previous%29)))
              (Development|ExecuteConsoleCommand (Utilities|String|Append "r.Lumen.ScreenProbeGather.MaxRayIntensity " (Utilities|String|ToString(Float) (Variables|Lumen|GetLumen%20Max%20Brightness))) 0)
              (Variables|TempSettings|SetLumen%20Max%20Brightness%20%28Previous%29 (Variables|Lumen|GetLumen%20Max%20Brightness))))
          (:then_1
            (Development|ExecuteConsoleCommand (Utilities|String|Append "r.Lumen.ScreenProbeGather.DownsampleFactor " (Utilities|String|ToString(Integer) (- 100 (Variables|Lumen|GetLumen%20Upsampling%20Amount)))) 0))
          (:then_2
            (Development|ExecuteConsoleCommand (Utilities|String|Append "r.Lumen.ScreenProbeGather.FullResolutionJitterWidth " (Utilities|String|ToString(Float) (- 1e+01 (Variables|Lumen|GetLumen%20Noise%20Jittering)))) 0))
          (:then_3
            (Development|ExecuteConsoleCommand (Utilities|String|Append "r.Lumen.ScreenProbeGather.SpatialFilterMaxRadianceHitAngle " (Utilities|String|ToString(Float) (Variables|Lumen|GetLumen%20Max%20Angle%20of%20Ray%20Hits))) 0))
          (:then_4
            (Development|ExecuteConsoleCommand (Utilities|String|Append "r.Lumen.ScreenProbeGather.SpatialFilterNumPasses " (Utilities|String|ToString(Integer) (Variables|Lumen|GetLumen%20Ray%20Num%20Passes))) 0))))
      (:then_1
        (bind _returnvalue (Actor|GetActorOfClass "/Game/M4/Blueprints/WorldLightingBP.WorldLightingBP_C" :!label _label))
        (Utilities|IsValid _returnvalue
          (:Is%20Valid
            (Variables|/Game/M4/Blueprints/WorldLightingBP.WorldLightingBP_C|SetEnable%20Lumen _returnvalue (Variables|Lumen|GetEnable%20Lumen))))))
    (else
      (Development|ExecuteConsoleCommand "r.Lumen.DiffuseIndirect.Allow 0" 0)
      (goto _label))))

(fn SetVirtualShadowMaps
  (bind _returnvalue (Development|GetConsoleVariableIntValue "r.Shadow.Virtual.Enable"))
  (Variables|TempSettings|SetEnable%20Virtual%20Shadow%20Maps%20%28Previous%29 (Math|Conversions|ToBoolean(Integer) _returnvalue))
  (if (== (Variables|VirtualShadowMaps|GetEnable%20Virtual%20Shadow%20Maps) (Variables|TempSettings|GetEnable%20Virtual%20Shadow%20Maps%20%28Previous%29))
    (Development|ExecuteConsoleCommand (Utilities|String|Append "r.Shadow.Virtual.SMRT.RayCountDirectional " (Utilities|String|ToString(Integer) (Variables|VirtualShadowMaps|GetVSM%20Directional%20Light%20Ray%20Count))) 0)
    (else
      (if (Variables|VirtualShadowMaps|GetEnable%20Virtual%20Shadow%20Maps)
        (Development|ExecuteConsoleCommand "r.Shadow.Virtual.Enable 1" 0)
        (else
          (Development|ExecuteConsoleCommand "r.Shadow.Virtual.Enable 0" 0)))
      (bind _returnvalue_2 (Actor|GetActorOfClass "/Game/M4/Blueprints/WorldLightingBP.WorldLightingBP_C"))
      (Utilities|IsValid _returnvalue_2
        (:Is%20Valid
          (Variables|/Game/M4/Blueprints/WorldLightingBP.WorldLightingBP_C|SetEnable%20Virtual%20Shadow%20Maps _returnvalue_2 (Variables|VirtualShadowMaps|GetEnable%20Virtual%20Shadow%20Maps)))))))

(fn ApplyVirtualShadowMapSettings)

(fn SetExtras
  (Development|ExecuteConsoleCommand (Utilities|String|Append "r.Tonemapper.Sharpen " (Utilities|String|ToString(Integer) (Variables|Extras|GetSharpen%20Scene))) 0)
  (if (< (Variables|Extras|GetIn%20Game%20Resolution%20Percentage) 99.0)
    (Development|ExecuteConsoleCommand "r.Editor.Viewport.OverridePIEScreenPercentage 0" 0)
    (Development|ExecuteConsoleCommand (Utilities|String|Append "r.ScreenPercentage " (Utilities|String|ToString(Float) (Variables|Extras|GetIn%20Game%20Resolution%20Percentage))) 0)))

(fn SetAnti-AliasingMode
  (Utilities|FlowControl|Sequence
    (:then_0
      (switch Utilities|FlowControl|Switch|SwitchonAntiAliasingSettings (Variables|AntiAliasing|GetAnti%20Aliasing%20Method)
        (:NewEnumerator0
          (Variables|AntiAliasing|SetAA%20Mode%20Number "0"))
        (:NewEnumerator1
          (Variables|AntiAliasing|SetAA%20Mode%20Number "1"))
        (:NewEnumerator2
          (Variables|AntiAliasing|SetAA%20Mode%20Number "2"))
        (:NewEnumerator3
          (Variables|AntiAliasing|SetAA%20Mode%20Number "3"))
        (:NewEnumerator4
          (Variables|AntiAliasing|SetAA%20Mode%20Number "4")))
      (Development|ExecuteConsoleCommand (Utilities|String|Append "r.AntiAliasingMethod " (Variables|AntiAliasing|GetAA%20Mode%20Number)) 0))
    (:then_1
      (Development|ExecuteConsoleCommand (Utilities|String|Append "r.TemporalAACurrentFrameWeight " (Utilities|String|ToString(Float) (Variables|AntiAliasing|GetTAA%20Current%20Frame%20Weight))) 0))))