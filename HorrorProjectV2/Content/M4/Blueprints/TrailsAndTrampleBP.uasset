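; Manager actor for terrain trail and foliage trample effects, with functions that place the volumes marking where they apply.
; BeginPlay converts both fade-out speeds into retention amounts in the PTMMPCVariables material parameter collection.
; Spawn functions create a scaled FoliageTrampleVolume or TerrainTrailVolume at the actor, enable box display and print placement hints.
; The construction script syncs every volume's cube visibility to ShowVolumeBoxes; Tick and capture events are empty.
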(event Custom|Start%20Capturing%20Grass%20Tramples)

(event Custom|Check%20and%20Show%20Volume%20Boxes
  (bind _show_volume_boxes (Variables|TrampleAndTrail-EnablingVolumes|GetShow%20Volume%20Boxes))
  (Utilities|FlowControl|Sequence
    (:then_0
      (bind _outactors (Actor|GetAllActorsOfClass "/Game/M4/Blueprints/SystemResources/Trails/EnablingVolumes/FoliageTrampleVolume.FoliageTrampleVolume_C"))
      (for _array_element _outactors
        (Rendering|SetVisibility (Variables|/Game/M4/Blueprints/SystemResources/Trails/EnablingVolumes/FoliageTrampleVolume.FoliageTrampleVolume_C|GetCube _array_element) _show_volume_boxes false)))
    (:then_1
      (bind _outactors_2 (Actor|GetAllActorsOfClass "/Game/M4/Blueprints/SystemResources/Trails/EnablingVolumes/TerrainTrailVolume.TerrainTrailVolume_C"))
      (for _array_element_2 _outactors_2
        (Rendering|SetVisibility (Variables|/Game/M4/Blueprints/SystemResources/Trails/EnablingVolumes/TerrainTrailVolume.TerrainTrailVolume_C|GetCube _array_element_2) _show_volume_boxes false)))))

(event EventBeginPlay
  (Rendering|Material|SetScalarParameterValue "/Game/M4/Blueprints/SystemResources/MagicMapMaterialBP/MPCs/PTM-MPC-Variables.PTM-MPC-Variables" "FoliageTrampleRetentionAmount_FadeOutSpeed" (- 1.0 (Variables|FoliageTrampleSettings|GetFoliage%20Interaction%20Fade%20Out%20Speed)) :!class /Script/Engine.KismetMaterialLibrary)
  (Rendering|Material|SetScalarParameterValue "/Game/M4/Blueprints/SystemResources/MagicMapMaterialBP/MPCs/PTM-MPC-Variables.PTM-MPC-Variables" "TrailRetentionAmount_FadeOutSpeed" (- 1.0 (* (Variables|TerrainDeformationSettings(Snow,Sand,Etc.)|GetTerrain%20Trail%20Fade%20Out%20Speed) 0.001)) :!class /Script/Engine.KismetMaterialLibrary))

(event EventTick
  (params (DeltaSeconds :type Float%20%28single-precision%29)))

(fn ConstructionScript
  (bind _show_volume_boxes (Variables|TrampleAndTrail-EnablingVolumes|GetShow%20Volume%20Boxes))
  (Utilities|FlowControl|Sequence
    (:then_0
      (bind _outactors (Actor|GetAllActorsOfClass "/Game/M4/Blueprints/SystemResources/Trails/EnablingVolumes/FoliageTrampleVolume.FoliageTrampleVolume_C"))
      (for _array_element _outactors
        (Rendering|SetVisibility (Variables|/Game/M4/Blueprints/SystemResources/Trails/EnablingVolumes/FoliageTrampleVolume.FoliageTrampleVolume_C|GetCube _array_element) _show_volume_boxes false)))
    (:then_1
      (bind _outactors_2 (Actor|GetAllActorsOfClass "/Game/M4/Blueprints/SystemResources/Trails/EnablingVolumes/TerrainTrailVolume.TerrainTrailVolume_C"))
      (for _array_element_2 _outactors_2
        (Rendering|SetVisibility (Variables|/Game/M4/Blueprints/SystemResources/Trails/EnablingVolumes/TerrainTrailVolume.TerrainTrailVolume_C|GetCube _array_element_2) _show_volume_boxes false)))))

(fn SpawnFoliageTrampleVolume
  (Variables|TrampleAndTrail-EnablingVolumes|SetShow%20Volume%20Boxes true)
  (Game|SpawnActorfromClass "/Game/M4/Blueprints/SystemResources/Trails/EnablingVolumes/FoliageTrampleVolume.FoliageTrampleVolume_C" (Math|Transform|MakeTransform (Transformation|GetActorLocation) "0, 0, 0" "200.000000,200.000000,50.000000") "Undefined" "OverrideRootScale" 0 0)
  (Development|PrintString "Now that the Foliage Trample Volume is spawned 
Align and scale it to where you want the effect in the world." true true "(R=0.002349,G=1.000000,B=0.000000,A=1.000000)" 2e+01)
  (CallFunction|CheckandShowVolumeBoxes))

(fn SpawnTerrainTrailVolume
  (Variables|TrampleAndTrail-EnablingVolumes|SetShow%20Volume%20Boxes true)
  (Game|SpawnActorfromClass "/Game/M4/Blueprints/SystemResources/Trails/EnablingVolumes/TerrainTrailVolume.TerrainTrailVolume_C" (Math|Transform|MakeTransform (Transformation|GetActorLocation) "0, 0, 0" "200.000000,200.000000,50.000000") "Undefined" "OverrideRootScale" 0 0)
  (Development|PrintString "Now that the Terrain Trail Volume is spawned 
Align and scale it to where you want the effect in the world." true true "(R=0.002349,G=1.000000,B=0.000000,A=1.000000)" 2e+01)
  (CallFunction|CheckandShowVolumeBoxes))