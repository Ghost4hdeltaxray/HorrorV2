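; BP_Door is an interactive door that player 0 toggles open and closed with the E key.
; Any actor overlap enables the door's input for that player, and end of overlap disables it, with no check on which actor overlaps.
; A FlipFlop alternates playing and reversing the DoorOperation timeline, which drives the door's relative yaw.
; Each toggle plays a different sound at the door's location.
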(event Collision|EventActorBeginOverlap
  (params (OtherActor :type Actor%20Object%20Reference))
  (Input|EnableInput (Game|GetPlayerController 0)))

(event Collision|EventActorEndOverlap
  (params (OtherActor :type Actor%20Object%20Reference))
  (Input|DisableInput (Game|GetPlayerController 0)))

(event Input|KeyboardEvents|E
  (params (Key :type Key%20Structure :default "None"))
  (bind _door (Variables|Default|GetDoor))
  (bind _returnvalue (Transformation|GetWorldLocation _door))
  (:Pressed
    (Utilities|FlowControl|FlipFlop
      (:A
        (Audio|PlaySoundatLocation "/Engine/VREditor/Sounds/UI/Camera_Shutter.Camera_Shutter" _returnvalue "0, 0, 0" 1.0 1.0 0.0 0 0 0 0)
        (bind _door_rotation (Timeline|Door%20Operation Play)
          (:Update
            (Transformation|SetRelativeRotation (Variables|Default|GetDoor) (Math|Rotator|MakeRotator 0.0 0.0 _door_rotation) false false))))
      (:B
        (Audio|PlaySoundatLocation "/Engine/VREditor/Sounds/UI/Dockable_Window_Close.Dockable_Window_Close" _returnvalue "0, 0, 0" 1.0 1.0 0.0 0 0 0 0)
        (Timeline|Door%20Operation Reverse)))))

(fn ConstructionScript)